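; BP_Button is a physical VR push button that sinks under the player's hand, with no action wired to a press.
; When a MYVRPawn component overlaps the Button, a fast looping timer maps that component's height above the Base to the Button's relative Z, clamped between BotPos and TopPos.
; Ending the overlap clears the timer and snaps the Button back to TopPos.
; The timer update also prints debug strings.
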(event `self.Button.OnComponentEndOverlap`
  (params (OverlappedComponent :type "PrimitiveComponent Object Reference") (OtherActor :type "Actor Object Reference") (OtherComp :type "PrimitiveComponent Object Reference") (OtherBodyIndex :type Integer))
  (if (`GameplayStatics.ObjectIsA` OtherActor "/Game/MYVRContent/MYVRPawn.MYVRPawn_C")
    (`KismetSystemLibrary.K2_ClearAndInvalidateTimerHandle` (stale `self.Button.OnComponentBeginOverlap` _returnvalue))
    (`SceneComponent.K2_SetRelativeLocation` (`self.Button`) (`KismetMathLibrary.MakeVector` 0.0 0.0 (`self.TopPos`)) false false)))

(event `self.Button.OnComponentBeginOverlap`
  (params (OverlappedComponent :type "PrimitiveComponent Object Reference") (OtherActor :type "Actor Object Reference") (OtherComp :type "PrimitiveComponent Object Reference") (OtherBodyIndex :type Integer) (bFromSweep :type Boolean) (SweepResult :type "HitResult Structure (by ref)"))
  (if (`GameplayStatics.ObjectIsA` OtherActor "/Game/MYVRContent/MYVRPawn.MYVRPawn_C")
    (set `self.Hand On Button` OtherComp)
    (bind _returnvalue (`KismetSystemLibrary.K2_SetTimerDelegate` (delegate `Hand Touching Button`) 0.01 true))))

(event `Hand Touching Button`
  (bind (_returnvalue_x _returnvalue_y _returnvalue_z) (`KismetMathLibrary.BreakVector` (`SceneComponent.K2_GetComponentLocation` (`self.Base`))))
  (bind (_returnvalue_x_2 _returnvalue_y_2 _returnvalue_z_2) (`KismetMathLibrary.BreakVector` (`SceneComponent.K2_GetComponentLocation` (`self.Hand On Button`))))
  (bind _returnvalue (+ (* (- _returnvalue_z_2 (+ _returnvalue_z 5.0)) 8.0) (`self.BotPos`)))
  (`KismetSystemLibrary.PrintString` "Hello")
  (if (<= _returnvalue (`self.BotPos`))
    (`KismetSystemLibrary.PrintString` "tru")
    (`SceneComponent.K2_SetRelativeLocation` (`self.Button`) (`KismetMathLibrary.MakeVector` 0.0 0.0 (`self.BotPos`)) false false)
    (else
      (`KismetSystemLibrary.PrintString` "false")
      (if (>= _returnvalue (`self.TopPos`))
        (`SceneComponent.K2_SetRelativeLocation` (`self.Button`) (`KismetMathLibrary.MakeVector` 0.0 0.0 (`self.TopPos`)) false false)
        (else
          (`SceneComponent.K2_SetRelativeLocation` (`self.Button`) (`KismetMathLibrary.MakeVector` 0.0 0.0 _returnvalue) false false))))))

(fn `UserConstructionScript`)