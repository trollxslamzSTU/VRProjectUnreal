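; BP_Note is a note actor that travels along a track spline and is destroyed when a stick hits it.
; If Active on BeginPlay, MoveNote plays a timeline scaled by Duration from StartOffset.
; Each update maps the timeline value to spline distance, applying local-space spline location and rotation to the actor.
; Box overlap with the BP_LeftStick or BP_RightStick found by GetActorOfClass destroys the note.
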(event `self.ReceiveBeginPlay`
  (if (`self.Active`)
    (`self.MoveNote`)))

(event `MoveNote`
  (bind _spline (`/Game/MYVRContent/Actors/BP_NoteTrack.Spline` (`self.NoteTrackRef`)))
  (bind _returnvalue (`KismetMathLibrary.Lerp` 0.0 (`SplineComponent.GetSplineLength` (`/Game/MYVRContent/Actors/BP_NoteTrack.Spline` (`self.NoteTrackRef`))) (`self.Movement Track`)))
  (`TimelineComponent.SetPlayRate` (`self.NoteTimeline`) (/ 1.0 (`self.Duration`)))
  (`TimelineComponent.SetNewTime` (`self.NoteTimeline`) (`self.StartOffset`))
  (bind (_direction _movementtrack) (`Timeline|NoteTimeline`)
    (:`Update`
      (set `self.Movement Track` _movementtrack)
      (`self.K2_SetActorLocationAndRotation` (`SplineComponent.GetLocationAtDistanceAlongSpline` _spline _returnvalue "Local") (`SplineComponent.GetRotationAtDistanceAlongSpline` _spline _returnvalue "Local")))))

(event `self.Box.OnComponentBeginOverlap`
  (params (OverlappedComponent :type "PrimitiveComponent Object Reference") (OtherActor :type "Actor Object Reference") (OtherComp :type "PrimitiveComponent Object Reference") (OtherBodyIndex :type Integer) (bFromSweep :type Boolean) (SweepResult :type "HitResult Structure (by ref)"))
  (bind _returnvalue (`GameplayStatics.GetActorOfClass` "/Game/MYVRContent/BP_LeftStick.BP_LeftStick_C"))
  (bind _returnvalue_2 (`GameplayStatics.GetActorOfClass` "/Game/MYVRContent/BP_RightStick.BP_RightStick_C"))
  (if (== _returnvalue OtherActor)
    (`self.K2_DestroyActor`)
    (elif (== _returnvalue_2 OtherActor)
      (`self.K2_DestroyActor`))))

(fn `UserConstructionScript`)