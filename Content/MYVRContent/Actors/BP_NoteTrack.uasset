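; BP_NoteTrack moves a set of actors around a spline in a continuous loop, triggering a random note each lap.
; The construction script spaces ActorOnSpline entries by OffsetBetween along the spline.
; A Timeline, rate-scaled by Duration, advances and wraps their distances, updating location and rotation.
; When the Timeline finishes, it restarts, picks a random BP_Note from the array and calls SpawnNote on it.
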(event `MoveNote`
  (bind _spline (`self.Spline`))
  (bind _distancealongspline (`self.DistanceAlongSpline`))
  (bind _noteref (`self.NoteRef`))
  (bind _returnvalue (`SplineComponent.GetSplineLength` (`self.Spline`)))
  (bind (_direction _alpha) (`Timeline|Timeline` :!via `PlayFromStart`)
    (:`Update`
      (for (_array_element _array_index) (`self.ActorOnSpline`)
        (bind _output_get (set `self.DistanceAlongSpline` (+ (* _array_index (`self.OffsetBetween`)) (`KismetMathLibrary.Lerp` 0.0 (`SplineComponent.GetSplineLength` (`self.Spline`)) _alpha))))
        (if (> _output_get _returnvalue)
          (set `self.DistanceAlongSpline` (- (`self.DistanceAlongSpline`) _returnvalue)))
        (`/Engine/EditorBlueprintResources/StandardMacros.IsValid` _array_element
          (:`Is Valid`
            (`self.K2_SetActorLocationAndRotation` _array_element (`SplineComponent.GetLocationAtDistanceAlongSpline` _spline _distancealongspline "World") (`SplineComponent.GetRotationAtDistanceAlongSpline` _spline _distancealongspline "World") false false)))))
    (:`Finished`
      (`self.MoveNote`)
      (`self.NoteGrab`)
      (`/Engine/EditorBlueprintResources/StandardMacros.IsValid` _noteref
        (:`Is Valid`
          (`/Game/MYVRContent/Actors/BP_Note.SpawnNote` _noteref))))))

(event `self.ReceiveBeginPlay`
  (`TimelineComponent.SetPlayRate` (`self.Timeline`) (/ 1.0 (`self.Duration`)))
  (`self.MoveNote`))

(event `NoteGrab`
  (bind _outitem (`KismetArrayLibrary.Array_Random` (`self.ActorOnSpline`)))
  (`/Engine/EditorBlueprintResources/StandardMacros.IsValid` _outitem
    (:`Is Valid`
      (bind _asbp_note (cast `/Game/MYVRContent/Actors/BP_Note` _outitem))
      (set `self.NoteRef` _asbp_note))))

(fn `UserConstructionScript`
  (bind _spline (`self.Spline`))
  (for (_array_element _array_index) (`self.ActorOnSpline`)
    (bind _returnvalue (* _array_index (`self.OffsetBetween`)))
    (`self.K2_SetActorLocationAndRotation` _array_element (`SplineComponent.GetLocationAtDistanceAlongSpline` _spline _returnvalue "World") (`SplineComponent.GetRotationAtDistanceAlongSpline` _spline _returnvalue "World") false false)))