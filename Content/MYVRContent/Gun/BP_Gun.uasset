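; VR gun actor that is assembled from separate parts and held by pistol grip, handguard or both.
; Overlap boxes snap matching stock, trigger, charging handle, magazine and bolt actors to BaseGun sockets, flagging their GrabComponents as JustSnapped.
; Grabbing disables physics and starts looping timers that position the gun from motion controllers, aiming grip-to-handguard when two-handed.
; Handguard-only holding still uses the PistolGrip's controller; releasing both restores physics.
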(event `self.StockBox.OnComponentBeginOverlap`
  (params (OverlappedComponent :type "PrimitiveComponent Object Reference") (OtherActor :type "Actor Object Reference") (OtherComp :type "PrimitiveComponent Object Reference") (OtherBodyIndex :type Integer) (bFromSweep :type Boolean) (SweepResult :type "HitResult Structure (by ref)"))
  (if (`GameplayStatics.ObjectIsA` OtherActor "/Game/MYVRContent/Gun/BP_Stock.BP_Stock_C")
    (`self.K2_AttachToComponent` OtherActor (`self.BaseGun`) "Stock" "SnapToTarget" "SnapToTarget" "SnapToTarget" true)
    (for _array_element (`self.K2_GetComponentsByClass` OtherActor "/Game/VRTemplate/Blueprints/GrabComponent.GrabComponent_C")
      (set `/Game/VRTemplate/Blueprints/GrabComponent.justSnapped` true _array_element))))

(event `self.TriggerBox.OnComponentBeginOverlap`
  (params (OverlappedComponent :type "PrimitiveComponent Object Reference") (OtherActor :type "Actor Object Reference") (OtherComp :type "PrimitiveComponent Object Reference") (OtherBodyIndex :type Integer) (bFromSweep :type Boolean) (SweepResult :type "HitResult Structure (by ref)"))
  (if (`GameplayStatics.ObjectIsA` OtherActor "/Game/MYVRContent/Gun/BP_Trigger.BP_Trigger_C")
    (`self.K2_AttachToComponent` OtherActor (`self.BaseGun`) "Trigger" "SnapToTarget" "SnapToTarget" "SnapToTarget" true)
    (for _array_element (`self.K2_GetComponentsByClass` OtherActor "/Game/VRTemplate/Blueprints/GrabComponent.GrabComponent_C")
      (set `/Game/VRTemplate/Blueprints/GrabComponent.justSnapped` true _array_element))))

(event `self.ChargingHandleBox.OnComponentBeginOverlap`
  (params (OverlappedComponent :type "PrimitiveComponent Object Reference") (OtherActor :type "Actor Object Reference") (OtherComp :type "PrimitiveComponent Object Reference") (OtherBodyIndex :type Integer) (bFromSweep :type Boolean) (SweepResult :type "HitResult Structure (by ref)"))
  (if (`GameplayStatics.ObjectIsA` OtherActor "/Game/MYVRContent/Gun/BP_ChargingHandle.BP_ChargingHandle_C")
    (`self.K2_AttachToComponent` OtherActor (`self.BaseGun`) "ChargingHandle" "SnapToTarget" "SnapToTarget" "SnapToTarget" true)
    (for _array_element (`self.K2_GetComponentsByClass` OtherActor "/Game/VRTemplate/Blueprints/GrabComponent.GrabComponent_C")
      (set `/Game/VRTemplate/Blueprints/GrabComponent.justSnapped` true _array_element))))

(event `self.MagazineBox.OnComponentBeginOverlap`
  (params (OverlappedComponent :type "PrimitiveComponent Object Reference") (OtherActor :type "Actor Object Reference") (OtherComp :type "PrimitiveComponent Object Reference") (OtherBodyIndex :type Integer) (bFromSweep :type Boolean) (SweepResult :type "HitResult Structure (by ref)"))
  (if (`GameplayStatics.ObjectIsA` OtherActor "/Game/MYVRContent/Gun/BP_Magazine.BP_Magazine_C")
    (`self.K2_AttachToComponent` OtherActor (`self.BaseGun`) "Magazine" "SnapToTarget" "SnapToTarget" "SnapToTarget" true)
    (for _array_element (`self.K2_GetComponentsByClass` OtherActor "/Game/VRTemplate/Blueprints/GrabComponent.GrabComponent_C")
      (set `/Game/VRTemplate/Blueprints/GrabComponent.justSnapped` true _array_element))))

(event `self.BoltBox.OnComponentBeginOverlap`
  (params (OverlappedComponent :type "PrimitiveComponent Object Reference") (OtherActor :type "Actor Object Reference") (OtherComp :type "PrimitiveComponent Object Reference") (OtherBodyIndex :type Integer) (bFromSweep :type Boolean) (SweepResult :type "HitResult Structure (by ref)"))
  (if (`GameplayStatics.ObjectIsA` OtherActor "/Game/MYVRContent/Gun/BP_Bolt.BP_Bolt_C")
    (`self.K2_AttachToComponent` OtherActor (`self.BaseGun`) "Bolt" "SnapToTarget" "SnapToTarget" "SnapToTarget" true)
    (for _array_element (`self.K2_GetComponentsByClass` OtherActor "/Game/VRTemplate/Blueprints/GrabComponent.GrabComponent_C")
      (set `/Game/VRTemplate/Blueprints/GrabComponent.justSnapped` true _array_element))))

(event `self.PistolGrip.OnDropped`
  (`KismetSystemLibrary.K2_ClearAndInvalidateTimerHandle` (stale `self.PistolGrip.OnGrabbed` _returnvalue))
  (if (and (not (`/Game/VRTemplate/Blueprints/GrabComponent.bIsHeld` (`self.Handguard`))) (not (`/Game/VRTemplate/Blueprints/GrabComponent.bIsHeld` (`self.PistolGrip`))))
    (`PrimitiveComponent.SetSimulatePhysics` (`self.BaseGun`) true)))

(event `self.PistolGrip.OnGrabbed`
  (bind _returnvalue (`KismetSystemLibrary.K2_SetTimerDelegate` (delegate `GripHeld`) 0.01 true))
  (`PrimitiveComponent.SetSimulatePhysics` (`self.BaseGun`) false))

(event `GripHeld`
  (bind _pistolgrip (`self.PistolGrip`))
  (bind _pistolgrip_2 (`self.PistolGrip`))
  (`|ExecutionSequence`
    (:`then_0`
      (if (not (`/Game/VRTemplate/Blueprints/GrabComponent.bIsHeld` (`self.Handguard`)))
        (`SceneComponent.K2_SetWorldRotation` (`self.BaseGun`) (`KismetMathLibrary.ComposeRotators` (`KismetMathLibrary.NegateRotator` (`SceneComponent.RelativeRotation` _pistolgrip)) (`SceneComponent.K2_GetComponentRotation` (`/Game/VRTemplate/Blueprints/GrabComponent.MotionControllerRef` _pistolgrip))) false false)))
    (:`then_1`
      (`SceneComponent.K2_SetWorldLocation` (`self.BaseGun`) (- (`SceneComponent.K2_GetComponentLocation` (`/Game/VRTemplate/Blueprints/GrabComponent.MotionControllerRef` _pistolgrip_2)) (- (`SceneComponent.K2_GetComponentLocation` _pistolgrip_2) (`SceneComponent.K2_GetComponentLocation` (`self.BaseGun`)))) false false))))

(event `self.Handguard.OnDropped`
  (`KismetSystemLibrary.K2_ClearAndInvalidateTimerHandle` (stale `self.Handguard.OnGrabbed` _returnvalue))
  (if (and (not (`/Game/VRTemplate/Blueprints/GrabComponent.bIsHeld` (`self.Handguard`))) (not (`/Game/VRTemplate/Blueprints/GrabComponent.bIsHeld` (`self.PistolGrip`))))
    (`PrimitiveComponent.SetSimulatePhysics` (`self.BaseGun`) true)))

(event `self.Handguard.OnGrabbed`
  (bind _returnvalue (`KismetSystemLibrary.K2_SetTimerDelegate` (delegate `HandguardHeld`) 0.01 true))
  (`PrimitiveComponent.SetSimulatePhysics` (`self.BaseGun`) false))

(event `HandguardHeld`
  (bind _pistolgrip (`self.PistolGrip`))
  (bind _pistolgrip_2 (`self.PistolGrip`))
  (if (`/Game/VRTemplate/Blueprints/GrabComponent.bIsHeld` (`self.PistolGrip`))
    (`SceneComponent.K2_SetWorldRotation` (`self.BaseGun`) (`KismetMathLibrary.FindLookAtRotation` (`SceneComponent.K2_GetComponentLocation` (`/Game/VRTemplate/Blueprints/GrabComponent.MotionControllerRef` (`self.PistolGrip`))) (`SceneComponent.K2_GetComponentLocation` (`/Game/VRTemplate/Blueprints/GrabComponent.MotionControllerRef` (`self.Handguard`)))) false false)
    (else
      (`SceneComponent.K2_SetWorldRotation` (`self.BaseGun`) (`KismetMathLibrary.ComposeRotators` (`KismetMathLibrary.NegateRotator` (`SceneComponent.RelativeRotation` _pistolgrip)) (`SceneComponent.K2_GetComponentRotation` (`/Game/VRTemplate/Blueprints/GrabComponent.MotionControllerRef` _pistolgrip))) false false)
      (`SceneComponent.K2_SetWorldLocation` (`self.BaseGun`) (- (`SceneComponent.K2_GetComponentLocation` (`/Game/VRTemplate/Blueprints/GrabComponent.MotionControllerRef` _pistolgrip_2)) (- (`SceneComponent.K2_GetComponentLocation` _pistolgrip_2) (`SceneComponent.K2_GetComponentLocation` (`self.BaseGun`)))) false false))))

(fn `UserConstructionScript`)